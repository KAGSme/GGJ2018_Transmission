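; Game state Blueprint that sets up a local two-player session on BeginPlay, with a guard and a top-down character.
; It creates the second player if missing and destroys both players' current pawns.
; Each PlayerStart tagged "guard" spawns a GuardChar for player 1; other starts spawn a TopDownCharacter for player 0.
; Each character is possessed and given its ParasiteController, and the top-down character then calls TransmitTo.
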(event `self.ReceiveBeginPlay`
  (bind _returnvalue (`GameplayStatics.GetPlayerController` 1))
  (bind _returnvalue_2 (`GameplayStatics.GetPlayerController` 0))
  (`/Engine/EditorBlueprintResources/StandardMacros.IsValid` (`GameplayStatics.GetPlayerController` 1)
    (:`Is Valid`
      _)
    (:`Is Not Valid`
      (`GameplayStatics.CreatePlayer` 1)))
  (`self.EnableInput` _returnvalue _returnvalue)
  (`self.K2_DestroyActor` (`Controller.K2_GetPawn` _returnvalue))
  (`self.K2_DestroyActor` (`Controller.K2_GetPawn` (`GameplayStatics.GetPlayerController` 0)))
  (bind _outactors (`GameplayStatics.GetAllActorsOfClass` "/Script/Engine.PlayerStart"))
  (for _array_element _outactors
    (if (== (`PlayerStart.PlayerStartTag` _array_element) "guard")
      (bind _returnvalue_3 (`|SpawnActorFromClass` "/Game/TopDownBP/Blueprints/GuardChar.GuardChar_C" (`self.GetTransform` _array_element) "Undefined" "OverrideRootScale"))
      (`Controller.Possess` _returnvalue _returnvalue_3)
      (bind _asparasite_controller (cast `/Game/TopDownBP/Blueprints/ParasiteController` _returnvalue))
      (set `/Game/TopDownBP/Blueprints/GuardChar.player` _asparasite_controller _returnvalue_3)
      (else
        (bind _returnvalue_4 (`|SpawnActorFromClass` "/Game/TopDownBP/Blueprints/TopDownCharacter.TopDownCharacter_C" (`self.GetTransform` _array_element) "Undefined" "OverrideRootScale"))
        (`Controller.Possess` _returnvalue_2 _returnvalue_4)
        (bind _asparasite_controller_2 (cast `/Game/TopDownBP/Blueprints/ParasiteController` _returnvalue_2))
        (set `/Game/TopDownBP/Blueprints/TopDownCharacter.PlayerController` _asparasite_controller_2 _returnvalue_4)
        (`/Game/TopDownBP/Blueprints/TopDownCharacter.TransmitTo` _returnvalue_4)))))

(fn `UserConstructionScript`)